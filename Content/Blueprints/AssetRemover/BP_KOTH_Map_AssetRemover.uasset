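; KOTH map helper actor that removes a list of soft-referenced level actors at BeginPlay, logging each one.
; On play it destroys its PostProcess component, then loads each asset blockingly and destroys it.
; The construction script's Preview enum can hide the targets' meshes or disable PostProcess.
; The M_RemovePreview material swap is gated on PostProcess being enabled just after it is disabled, so it never runs as written.
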(event `self.ReceiveBeginPlay`
  (`ActorComponent.K2_DestroyComponent` (`self.PostProcess`))
  (for _array_element (`self.Assets`)
    (bind _returnvalue (`KismetSystemLibrary.LoadAsset_Blocking` _array_element))
    (bind _asactor (cast `Actor` _returnvalue))
    (`self.K2_DestroyActor` _asactor)
    (`KismetSystemLibrary.PrintString` (`KismetStringLibrary.Concat_StrStr` "KOTH Asset Remover Cleared Asset:" (`KismetSystemLibrary.GetDisplayName` _asactor)))))

(fn `UserConstructionScript`
  (if (`|EnumEquality` (`self.Preview`) "NewEnumerator1")
    (bind _output_get (set `PostProcessComponent.bEnabled` false (`self.PostProcess`)))
    (if _output_get
      (for _array_element (`self.Assets`)
        (bind _returnvalue (`KismetSystemLibrary.LoadAsset_Blocking` _array_element))
        (bind _asactor (cast `Actor` _returnvalue))
        (for _array_element_2 (`self.K2_GetComponentsByClass` _asactor "/Script/Engine.MeshComponent")
          (for (_ _array_index) (`MeshComponent.GetMaterials` _array_element_2)
            (`PrimitiveComponent.SetMaterial` _array_element_2 _array_index "/KingOfTheHill/Blueprints/AssetRemover/M_RemovePreview.M_RemovePreview")))))
    (elif (`|EnumEquality` (`self.Preview`) "NewEnumerator2")
      (for _array_element_3 (`self.Assets`)
        (bind _returnvalue_2 (`KismetSystemLibrary.LoadAsset_Blocking` _array_element_3))
        (bind _asactor_2 (cast `Actor` _returnvalue_2))
        (for _array_element_4 (`self.K2_GetComponentsByClass` _asactor_2 "/Script/Engine.MeshComponent")
          (`SceneComponent.SetVisibility` _array_element_4 false false))))))