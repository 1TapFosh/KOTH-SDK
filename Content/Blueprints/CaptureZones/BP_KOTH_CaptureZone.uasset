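; BP_KOTH_CaptureZone is a King of the Hill capture zone with a moving priority area inside it.
; On the authority it registers itself with the KOTH ruleset at BeginPlay.
; StartZone triggers UpdateLocation immediately and on a looping ZoneMoveInterval timer, while Tick glides the Prio component toward its target at constant speed.
; Query functions for players and bots, radius OnReps and UpdateLocation have empty bodies here.
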(event `StartZone`
  (bind _zone_move_interval (`self.Zone Move Interval`))
  (`KismetSystemLibrary.K2_ClearAndInvalidateTimerHandle` (`self.Prio Timer Handle`))
  (`/Engine/EditorBlueprintResources/StandardMacros.IsValid` (`self.KOTH Ruleset`)
    (:`Is Valid`
      (if (> _zone_move_interval 0.0)
        (bind _returnvalue (`KismetSystemLibrary.K2_SetTimerDelegate` (delegate `Update Prio Location`) _zone_move_interval true)) ; zone will shift positions every 5 min
        (set `self.Prio Timer Handle` _returnvalue)
        (`self.Update Prio Location`)))))

(event `Update Prio Location`
  (`self.Update Location`))

(event `self.ReceiveBeginPlay`
  (`/Engine/EditorBlueprintResources/ActorMacros.Switch Has Authority`
    (:`Authority`
      (bind _outruleset (`/KingOfTheHill/Blueprints/BPFL_KOTH.GetKOTHRuleset`))
      (bind _output_get (set `self.KOTH Ruleset` _outruleset))
      (`/Engine/EditorBlueprintResources/StandardMacros.IsValid` _output_get
        (:`Is Valid`
          (set `/KingOfTheHill/Blueprints/BP_Ruleset_KOTH.Zone` self _output_get))))))

(event `self.ReceiveTick`
  (params (DeltaSeconds :type "Float (single-precision)"))
  (`SceneComponent.K2_SetRelativeLocation` (`self.Prio`) (`KismetMathLibrary.VInterpTo_Constant` (`SceneComponent.RelativeLocation` (`self.Prio`)) (`self.New Target Location`) DeltaSeconds (`self.New Rate`)) false false))

(fn `GetBotsInPriorityZone`
  (locals (CurrentActor :type "Actor Object Reference") (L_Bots :type "Array of /KingOfTheHill/Blueprints/Bots/BotSoldiers/SquidBot_KOTH Object Reference")))

(fn `GetBotsInZone`
  (locals (CurrentActor :type "Actor Object Reference") (L_Bots :type "Array of /KingOfTheHill/Blueprints/Bots/BotSoldiers/SquidBot_KOTH Object Reference")))

(fn `GetPlayersInPriorityZone`
  (params (bIncludeVehicles :type Boolean))
  (locals (L_PlayersToReward :type "Array of /KingOfTheHill/Blueprints/BP_PlayerController_KOTH Object Reference") (CurrentActor :type "Actor Object Reference")))

(fn `GetPlayersInZone`
  (params (bIncludeVehicles :type Boolean) (bPrioIncludeVehicles :type Boolean))
  (locals (L_PlayersToReward :type "Array of /KingOfTheHill/Blueprints/BP_PlayerController_KOTH Object Reference") (CurrentActor :type "Actor Object Reference")))

(fn `OnRep_Prio Radius`)

(fn `OnRep_Radius`)

(fn `Update Location`
  (locals (`Attempt Location` :type "Vector Structure" :default (0.0 0.0 0.0)) (`Zone Valid` :type Boolean) (`Attempt Count` :type Integer)))

(fn `UserConstructionScript`
  (`SceneComponent.K2_SetWorldRotation` :`self` (`self.CaptureZone`)) ; like why do you need to rotate a sphere anyways
)